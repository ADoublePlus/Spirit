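; BP_Meteor is a meteor power actor that explodes on impact and damages BP_Enemy1 actors.
; A blocking hit on its Box collision spawns an explosion particle and sound at the impact point, then destroys the meteor.
; Box overlaps apply a small amount of damage to BP_Enemy1 only and destroy that enemy if its Health is depleted, leaving the meteor intact.
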(event OnComponentHit(Box)
  (params (HitComponent :type Primitive%20Component%20Object%20Reference) (OtherActor :type Actor%20Object%20Reference) (OtherComp :type Primitive%20Component%20Object%20Reference) (NormalImpulse :type Vector :default "0, 0, 0") (Hit :type Hit%20Result%20Structure%20%28by%20ref%29))
  (bind (_bblockinghit _binitialoverlap _time _distance _location _impactpoint _normal _impactnormal _physmat _hitactor) (Collision|BreakHitResult Hit))
  (Effects|SpawnEmitteratLocation "/Game/StarterContent/Particles/P_Explosion.P_Explosion" _impactpoint (.rotation (Transformation|GetActorTransform _hitactor)))
  (Audio|PlaySoundatLocation "/Game/StarterContent/Audio/Explosion_Cue.Explosion_Cue" _impactpoint "0, 0, 0" 1.0 1.0 0.0 0 0 0)
  (Actor|DestroyActor))

(event OnComponentBeginOverlap(Box)
  (params (OverlappedComponent :type Primitive%20Component%20Object%20Reference) (OtherActor :type Actor%20Object%20Reference) (OtherComp :type Primitive%20Component%20Object%20Reference) (OtherBodyIndex :type Integer) (bFromSweep :type Boolean) (SweepResult :type Hit%20Result%20Structure%20%28by%20ref%29))
  (bind _asbp_enemy_1 (Utilities|Casting|CastToBP_Enemy1 OtherActor))
  (Game|Damage|ApplyDamage _asbp_enemy_1 0.3 0 0)
  (if (<= (Variables|/Game/FireballCharacter/BP_Enemy1.BP_Enemy1_C|GetHealth _asbp_enemy_1) 0.0)
    (Actor|DestroyActor _asbp_enemy_1)))

(event EventBeginPlay)

(event Collision|EventActorBeginOverlap
  (params (OtherActor :type Actor%20Object%20Reference)))

(event EventTick
  (params (DeltaSeconds :type Float%20%28single-precision%29)))

(fn ConstructionScript)