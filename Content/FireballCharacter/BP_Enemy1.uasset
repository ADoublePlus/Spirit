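; BP_Enemy1 is an enemy pawn that chases and damages the player's BP_FireChar.
; PawnSensing detects the player and starts an AI move toward them, and overlapping the Box component subtracts health from the player, calling Death at zero.
; Incoming damage lowers the enemy's own Health and refreshes an EnemyHealth widget, which is linked to the enemy on BeginPlay.
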(event OnSeePawn(PawnSensing)
  (params (Pawn :type Pawn%20Object%20Reference))
  (bind _asbp_fire_char (Utilities|Casting|CastToBP_FireChar Pawn))
  (AI|AIMoveTo self "0, 0, 0" _asbp_fire_char 5.0 false))

(event OnComponentBeginOverlap(Box)
  (params (OverlappedComponent :type Primitive%20Component%20Object%20Reference) (OtherActor :type Actor%20Object%20Reference) (OtherComp :type Primitive%20Component%20Object%20Reference) (OtherBodyIndex :type Integer) (bFromSweep :type Boolean) (SweepResult :type Hit%20Result%20Structure%20%28by%20ref%29))
  (bind _asbp_fire_char (Utilities|Casting|CastToBP_FireChar OtherActor))
  (bind _output_get (Variables|/Game/FireballCharacter/BP_FireChar.BP_FireChar_C|SetHealth _asbp_fire_char (- (Variables|/Game/FireballCharacter/BP_FireChar.BP_FireChar_C|GetHealth _asbp_fire_char) 0.3)))
  (if (<= _output_get 0.0)
    (Default|Death _asbp_fire_char)))

(event EventBeginPlay
  (bind _asenemy_health (Utilities|Casting|CastToEnemyHealth (UserInterface|GetUserWidgetObject (Variables|Default|GetEnemyHB))))
  (bind _output_get (Variables|Default|SetEnemyHealthBar _asenemy_health))
  (Variables|/Game/FireballCharacter/EnemyHealth.EnemyHealth_C|SetEnemy _output_get self)
  (Default|UpdateHealth _output_get))

(event Collision|EventActorBeginOverlap
  (params (OtherActor :type Actor%20Object%20Reference)))

(event EventTick
  (params (DeltaSeconds :type Float%20%28single-precision%29)))

(event Game|Damage|EventAnyDamage
  (params (Damage :type Float%20%28single-precision%29) (DamageType :type Damage%20Type%20Object%20Reference) (InstigatedBy :type Controller%20Object%20Reference) (DamageCauser :type Actor%20Object%20Reference))
  (Variables|Default|SetHealth (- (Variables|Default|GetHealth) Damage))
  (Default|UpdateHealth (Variables|Default|GetEnemyHealthBar)))

(fn ConstructionScript)

(fn OnRepEnemyHealthBar)