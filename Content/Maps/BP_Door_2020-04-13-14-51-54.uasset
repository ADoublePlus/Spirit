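; Door actor Blueprint that opens once when its OpenDoor event fires while the door is closed.
; BeginPlay caches the player character, cast to Player, for use when opening.
; OpenDoor clears the closed flag, stores the dot product of the normalized player-to-door direction and the Scene component's forward vector to record the player's side, then plays the OpenDoor_TL timeline.
; The graph shows no timeline update logic or closing path.
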(event Custom|OpenDoor
  (bind _scene (Variables|Default|GetScene))
  (if (Variables|Default|GetisDoorClosed)
    (Variables|Default|SetisDoorClosed false)
    (Variables|Default|SetDotProduct (Math|Vector|DotProduct (Math|Vector|Normalize (- (Transformation|GetWorldLocation _scene) (Transformation|GetActorLocation (Variables|Default|GetPlayerRef)))) (Math|Vector|GetForwardVector _scene)))
    (Timeline|OpenDoor_TL Play)))

(event EventBeginPlay
  (bind _asplayer (Utilities|Casting|CastToPlayer (Game|GetPlayerCharacter 0)))
  (Variables|Default|SetPlayerRef _asplayer))

(fn ConstructionScript)