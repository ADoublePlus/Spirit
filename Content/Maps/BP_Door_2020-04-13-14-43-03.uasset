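; BP_Door is a door Blueprint that so far only prints a facing test against the player, with an empty OpenDoor event.
; BeginPlay caches player character 0 as a Player reference.
; Every Tick, it takes the dot product of the normalized player-to-door direction and the Scene component's forward vector, showing which side the player is on.
; The result prints on screen for one frame as debug output.
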(event Custom|OpenDoor)

(event EventBeginPlay
  (bind _asplayer (Utilities|Casting|CastToPlayer (Game|GetPlayerCharacter 0)))
  (Variables|Default|SetPlayerRef _asplayer))

(event EventTick
  (params (DeltaSeconds :type Float%20%28single-precision%29))
  (bind _scene (Variables|Default|GetScene))
  (Development|PrintString (Utilities|String|ToString(Float) (Math|Vector|DotProduct (Math|Vector|Normalize (- (Transformation|GetWorldLocation _scene) (Transformation|GetActorLocation (Variables|Default|GetPlayerRef)))) (Math|Vector|GetForwardVector _scene))) true true "(R=0.000000,G=0.660000,B=1.000000,A=1.000000)" DeltaSeconds))

(fn ConstructionScript)