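; Door actor that swings open or shut on its OpenDoor event, turning toward a side chosen by where the player stands.
; The dot product of the player-to-door direction and the door's forward vector picks positive or negative 90 degree yaw.
; A timeline lerps the door's relative rotation; later calls reverse it, and the door counts as closed only once that reverse finishes.
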(event Custom|OpenDoor
  (bind _scene (Variables|Default|GetScene))
  (if (Variables|Default|GetisDoorClosed)
    (Variables|Default|SetisDoorClosed false)
    (Variables|Default|SetDotProduct (Math|Vector|DotProduct (Math|Vector|Normalize (- (Transformation|GetWorldLocation _scene) (Transformation|GetActorLocation (Variables|Default|GetPlayerRef)))) (Math|Vector|GetForwardVector _scene)))
    (bind (_direction _alpha) (Timeline|OpenDoor_TL Play)
      (:Update
        (Transformation|SetRelativeRotation (Variables|Default|GetDoor) (Math|Rotator|MakeRotator 0.0 0.0 (Math|Float|Lerp 0.0 (Math|Float|SelectFloat 9e+01 -9e+01 (>= (Variables|Default|GetDotProduct) 0.0)) _alpha)) false false))
      (:Finished
        (switch Utilities|FlowControl|Switch|SwitchonETimelineDirection _direction
          (:Backward
            (Variables|Default|SetisDoorClosed true)))))
    (else
      (Timeline|OpenDoor_TL Reverse))))

(event EventBeginPlay
  (bind _asplayer (Utilities|Casting|CastToPlayer (Game|GetPlayerCharacter 0)))
  (Variables|Default|SetPlayerRef _asplayer))

(fn ConstructionScript)