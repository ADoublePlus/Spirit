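; Enemy NPC that takes fire-spell hits, shows a widget health bar and hurts the player through melee.
; Overlapping flame projectiles or vortexes spawn explosions, lower Health and destroy the NPC at zero, without refreshing the bar.
; AnyDamage refreshes the bar but sets Health to Damage minus Health, reversing the usual subtraction.
; MeleeAttack only plays a montage; Box overlap directly reduces Player health.
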(event OnComponentBeginOverlap(Box)
  (params (OverlappedComponent :type Primitive%20Component%20Object%20Reference) (OtherActor :type Actor%20Object%20Reference) (OtherComp :type Primitive%20Component%20Object%20Reference) (OtherBodyIndex :type Integer) (bFromSweep :type Boolean) (SweepResult :type Hit%20Result%20Structure%20%28by%20ref%29))
  (bind _asplayer (Utilities|Casting|CastToPlayer OtherActor))
  (Variables|/Game/Character/Humanoid/Player.Player_C|SetHealth _asplayer (- (Variables|/Game/Character/Humanoid/Player.Player_C|GetHealth _asplayer) 0.3)))

(event Collision|EventActorBeginOverlap
  (params (OtherActor :type Actor%20Object%20Reference))
  (Utilities|FlowControl|Sequence
    (:then_0
      (bind _asflame_projectile (Utilities|Casting|CastToFlameProjectile OtherActor))
      (Effects|SpawnEmitteratLocation "/Game/StarterContent/Particles/P_Explosion.P_Explosion" (Transformation|GetActorLocation _asflame_projectile))
      (bind _output_get (Variables|Default|SetHealth (- (Variables|Default|GetHealth) 0.25)))
      (if (<= _output_get 0.0)
        (Actor|DestroyActor _asflame_projectile)
        (Actor|DestroyActor)
        (else
          (Actor|DestroyActor _asflame_projectile))))
    (:then_1
      (bind _asflame_vortex (Utilities|Casting|CastToFlameVortex OtherActor))
      (Effects|SpawnEmitteratLocation "/Game/StarterContent/Particles/P_Explosion.P_Explosion" (Transformation|GetActorLocation _asflame_vortex))
      (bind _output_get_2 (Variables|Default|SetHealth (- (Variables|Default|GetHealth) 0.3)))
      (if (<= _output_get_2 0.0)
        (Actor|DestroyActor)))))

(event EventBeginPlay
  (bind _asenemy_health (Utilities|Casting|CastToEnemyHealth (UserInterface|GetUserWidgetObject (Variables|Default|GetEnemyHealthBar))))
  (bind _output_get (Variables|Default|SetAiHealthBarWidget _asenemy_health))
  (Variables|/Game/AI/NPC/EnemyHealth.EnemyHealth_C|SetEnemy _output_get self)
  (Default|UpdateHealth _output_get))

(event EventMeleeAttack
  (Animation|Montage|PlayMontage (Variables|Character|GetMesh) "/Game/AI/NPC/Attack_PrimaryA_Montage.Attack_PrimaryA_Montage"))

(event Game|Damage|EventAnyDamage
  (params (Damage :type Float%20%28single-precision%29) (DamageType :type Damage%20Type%20Object%20Reference) (InstigatedBy :type Controller%20Object%20Reference) (DamageCauser :type Actor%20Object%20Reference))
  (Variables|Default|SetHealth (- Damage (Variables|Default|GetHealth)))
  (Default|UpdateHealth (Variables|Default|GetAiHealthBarWidget)))

(fn ConstructionScript)